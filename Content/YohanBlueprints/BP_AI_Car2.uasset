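; AI-driven race car that follows a BP_Path spline once the player controller flags the race start.
; Each tick it steers toward a spline point projected ahead along the tangent, with look-ahead distance scaled by speed.
; Above a speed threshold, a forward line trace triggers braking logic: overlapped BP_CornerIndex actors select sharp-right or hairpin handling, otherwise brake input is mapped from hit distance.
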(event `self.ReceiveTick`
  (params (DeltaSeconds :type "Float (single-precision)"))
  (bind (_frontpathtracehitresult_bblockinghit _frontpathtracehitresult_binitialoverlap _frontpathtracehitresult_time _frontpathtracehitresult_distance) (`GameplayStatics.BreakHitResult` (`self.FrontPathTraceHitResult`)))
  (if (`/Game/VehicleTemplate/Blueprints/VehiclePlayerController.RaceStart` (stale `self.ReceiveBeginPlay` _output_get))
    (bind _outactors (`GameplayStatics.GetAllActorsOfClass` "/Game/YohanBlueprints/BP_Path.BP_Path_C"))
    (bind _steering (`self.GetPath` _outactors))
    (`ChaosVehicleMovementComponent.SetSteeringInput` (`self.VehicleMovementComponent`) _steering)
    (`self.SpeedLimiter` 0.6
      (:`UnderSpeedLimit`
        (`self.SetInput` 0.5))
      (:`OverSpeedLimit`
        (`self.LineTracer`)
        (if (`self.FrontPathTraceHit`)
          (bind _corner (`self.GetCorner`)
            (:`InCorner`
              (bind _asbp_corner_index (cast `/Game/YohanBlueprints/BP_CornerIndex` _corner))
              (switch `/Game/YohanBlueprints/E_TurnIndex` (`/Game/YohanBlueprints/BP_CornerIndex.TurnIndex` _asbp_corner_index)
                (:`NewEnumerator0`
                  (`self.SpeedLimiter` 0.6
                    (:`UnderSpeedLimit`
                      (`self.SetInput` 0.5))
                    (:`OverSpeedLimit`
                      (`self.SetInput` 0.0 1.0))))
                (:`NewEnumerator1`
                  (`self.SpeedLimiter` 0.6
                    (:`UnderSpeedLimit`
                      (`self.SetInput` 0.5))
                    (:`OverSpeedLimit`
                      (`self.SetInput` 0.0 1.0))))))
            (:`NotInCorner`
              (`self.SetInput` 0.5 (`KismetMathLibrary.MapRangeClamped` _frontpathtracehitresult_distance 0.0 1.0 0.0 1500.0))))
          (else
            (`self.SetInput` 0.5)))))))

(event `self.ReceiveBeginPlay`
  (bind _asvehicle_player_controller (cast `/Game/VehicleTemplate/Blueprints/VehiclePlayerController` (`GameplayStatics.GetPlayerController` 0)))
  (bind _output_get (set `self.PlayerControllerReference` _asvehicle_player_controller)))

(fn `GetCurrentCarSpeed`
  (returns (Speed :type "Float (double-precision)"))
  (return (* (`ChaosVehicleMovementComponent.GetForwardSpeed` (`self.VehicleMovementComponent`)) 0.036)))

(fn `GetPath`
  (params (Path :type "Array of /Game/YohanBlueprints/BP_Path Object Reference"))
  (returns (Steering :type "Float (double-precision)"))
  (bind _returnvalue (`self.K2_GetActorLocation`))
  (bind _spline (`/Game/YohanBlueprints/BP_Path.Spline` (`|GetArrayItem` Path)))
  (bind (_returnvalue_roll _returnvalue_pitch _returnvalue_yaw) (`KismetMathLibrary.BreakRotator` (`KismetMathLibrary.NormalizedDeltaRotator` (`KismetMathLibrary.FindLookAtRotation` _returnvalue (`SplineComponent.FindLocationClosestToWorldLocation` _spline (+ (* (`KismetMathLibrary.Normal` (`SplineComponent.FindTangentClosestToWorldLocation` _spline _returnvalue "World")) (`KismetMathLibrary.MapRangeClamped` (`self.GetCurrentCarSpeed`) 20.0 80.0 50.0 500.0)) _returnvalue) "World")) (`self.K2_GetActorRotation`))))
  (return (`KismetMathLibrary.MapRangeClamped` _returnvalue_yaw -90.0 90.0 -1.0 1.0)))

(fn `LineTracer`
  (bind _pathtracestartpoint (`self.PathTraceStartPoint`))
  (bind _returnvalue (`SceneComponent.K2_GetComponentLocation` _pathtracestartpoint))
  (bind (_outhit _returnvalue_2) (`KismetSystemLibrary.LineTraceSingle` :`Start` _returnvalue :`End` (+ _returnvalue (* (`SceneComponent.GetForwardVector` _pathtracestartpoint) 1500.0)) :`TraceChannel` "TraceTypeQuery1" :`DrawDebugType` "ForOneFrame"))
  (set `self.FrontPathTraceHitResult` _outhit)
  (set `self.FrontPathTraceHit` _returnvalue_2))

(fn `SetInput`
  (params (Throttle :type "Float (single-precision)") (Brake :type "Float (single-precision)"))
  (`ChaosVehicleMovementComponent.SetThrottleInput` (`self.VehicleMovementComponent`) Throttle)
  (`ChaosVehicleMovementComponent.SetBrakeInput` (`self.VehicleMovementComponent`) Brake))

(fn `UserConstructionScript`)
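; BP_Checkpoint is a one-shot, numbered checkpoint that registers when the player vehicle passes through it in the correct direction.
; When the vehicle leaves the trigger, a dot product of its velocity and the arrow's forward vector confirms the direction.
; A valid pass broadcasts CheckpointCleared with the checkpoint number, hides the trigger and Niagara effect, and turns off the trigger's overlap events.
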(event `self.Trigger.OnComponentEndOverlap`
  (params (OverlappedComponent :type "PrimitiveComponent Object Reference") (OtherActor :type "Actor Object Reference") (OtherComp :type "PrimitiveComponent Object Reference") (OtherBodyIndex :type Integer))
  (bind _trigger (`self.Trigger`))
  (bind _asbp_vehicle_player (cast `/Game/YohanBlueprints/BP_VehiclePlayer` OtherActor))
  (if (> (`KismetMathLibrary.Dot_VectorVector` (`self.GetVelocity` _asbp_vehicle_player) (`KismetMathLibrary.Conv_RotatorToVector` (`SceneComponent.K2_GetComponentRotation` (`self.Arrow`)))) 0.0)
    (`self.CheckpointCleared` (`self.CheckpointNumber`))
    (`SceneComponent.SetHiddenInGame` _trigger true false)
    (`SceneComponent.SetHiddenInGame` (`self.Niagara`) true false)
    (set `PrimitiveComponent.bGenerateOverlapEvents` false _trigger)))

(fn `UserConstructionScript`)
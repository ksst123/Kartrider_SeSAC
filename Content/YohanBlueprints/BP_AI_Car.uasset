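; BP_AI_Car is an AI vehicle that drives itself along the spline of the first BP_Path actor found in the level.
; BeginPlay sets full throttle, and Tick looks up the path actors every frame to update steering.
; GetPath projects a look-ahead point along the spline tangent, snaps it to the spline, and maps the yaw error to clamped steering input.
; GetPath_0 is an unused duplicate of GetPath.
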(event `self.ReceiveTick`
  (params (DeltaSeconds :type "Float (single-precision)"))
  (bind _outactors (`GameplayStatics.GetAllActorsOfClass` "/Game/YohanBlueprints/BP_Path.BP_Path_C"))
  (bind _steering (`self.GetPath` _outactors))
  (`ChaosVehicleMovementComponent.SetSteeringInput` (`self.VehicleMovementComponent`) _steering))

(event `self.ReceiveBeginPlay`
  (`|ExecutionSequence`
    (:`then_1`
      (`ChaosVehicleMovementComponent.SetThrottleInput` (`self.VehicleMovementComponent`) 1.0))))

(fn `GetPath`
  (params (Splines :type "Array of /Game/YohanBlueprints/BP_Path Object Reference"))
  (returns (Steering :type "Float (double-precision)"))
  (bind _returnvalue (`self.K2_GetActorLocation`))
  (bind _spline (`/Game/YohanBlueprints/BP_Path.Spline` (`|GetArrayItem` Splines)))
  (bind (_returnvalue_roll _returnvalue_pitch _returnvalue_yaw) (`KismetMathLibrary.BreakRotator` (`KismetMathLibrary.NormalizedDeltaRotator` (`KismetMathLibrary.FindLookAtRotation` _returnvalue (`SplineComponent.FindLocationClosestToWorldLocation` _spline (+ (* (`KismetMathLibrary.Normal` (`SplineComponent.FindTangentClosestToWorldLocation` _spline _returnvalue "World")) (`self.Num`)) _returnvalue) "World")) (`self.K2_GetActorRotation`))))
  (return (`KismetMathLibrary.MapRangeClamped` _returnvalue_yaw -90.0 90.0 -1.0 1.0)))

(fn `GetPath_0`
  (params (Splines :type "Array of /Game/YohanBlueprints/BP_Path Object Reference"))
  (returns (Steering :type "Float (double-precision)"))
  (bind _returnvalue (`self.K2_GetActorLocation`))
  (bind _spline (`/Game/YohanBlueprints/BP_Path.Spline` (`|GetArrayItem` Splines)))
  (bind (_returnvalue_roll _returnvalue_pitch _returnvalue_yaw) (`KismetMathLibrary.BreakRotator` (`KismetMathLibrary.NormalizedDeltaRotator` (`KismetMathLibrary.FindLookAtRotation` _returnvalue (`SplineComponent.FindLocationClosestToWorldLocation` _spline (+ (* (`KismetMathLibrary.Normal` (`SplineComponent.FindTangentClosestToWorldLocation` _spline _returnvalue "World")) (`self.Num`)) _returnvalue) "World")) (`self.K2_GetActorRotation`))))
  (return (`KismetMathLibrary.MapRangeClamped` _returnvalue_yaw -90.0 90.0 -1.0 1.0)))

(fn `UserConstructionScript`)
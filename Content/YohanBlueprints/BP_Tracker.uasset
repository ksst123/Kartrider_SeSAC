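; BP_Tracker runs a checkpoint lap race, pushing lap and time settings to the VehiclePlayerController at BeginPlay.
; It numbers the Checkpoints array, activates the first, binds each one's cleared callback and starts level music.
; Each clear activates the next checkpoint and updates the respawn transform, while the last one checks laps against MaxLap.
; A completed race restarts through the controller, which holds the race state.
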(event `self.ReceiveBeginPlay`
  (bind _asvehicle_player_controller (cast `/Game/VehicleTemplate/Blueprints/VehiclePlayerController` (`GameplayStatics.GetPlayerController` 0)))
  (set `self.ControllerReference` _asvehicle_player_controller)
  (`self.ApplySettings`)
  (`self.StartSequence`))

(event `ApplySettings`
  (bind _controllerreference (`self.ControllerReference`))
  (set `/Game/VehicleTemplate/Blueprints/VehiclePlayerController.MaxLap` (`self.MaxLap`) _controllerreference)
  (`self.UpdateTimes`)
  (`/Game/VehicleTemplate/Blueprints/VehiclePlayerController.StartGameSetup` _controllerreference))

(event `StartSequence`
  (bind _checkpoints (`self.Checkpoints`))
  (for (_array_element _array_index) (`self.Checkpoints`)
    (set `/Game/YohanBlueprints/BP_Checkpoint.CheckpointNumber` (+ _array_index 1) _array_element)
    (set `self.TotalCheckpoints` (`KismetArrayLibrary.Array_Length` _checkpoints))
    (`self.ActivateCheckpoint` (`|GetArrayItem` _checkpoints))
    (for _array_element_2 (`self.Checkpoints`)
      (add `/Game/YohanBlueprints/BP_Checkpoint.CheckpointCleared` _array_element_2 (delegate `Checkpoint Cleared`))
      (`AudioComponent.Play` (`AmbientSound.AudioComponent` (`self.LevelMusic`)) 0.0))))

(event `Checkpoint Cleared`
  (params (NextCheckpoint :type Integer))
  (bind _controllerreference (`self.ControllerReference`))
  (`self.LapCheck` NextCheckpoint)
  (if (`/Game/VehicleTemplate/Blueprints/VehiclePlayerController.RaceComplete` _controllerreference)
    (`/Game/VehicleTemplate/Blueprints/VehiclePlayerController.Restart` _controllerreference)))

(fn `ActivateCheckpoint`
  (params (NextCheckpoint :type "/Game/YohanBlueprints/BP_Checkpoint Object Reference"))
  (bind _trigger (`/Game/YohanBlueprints/BP_Checkpoint.Trigger` NextCheckpoint))
  (`SceneComponent.SetHiddenInGame` _trigger false false)
  (`SceneComponent.SetHiddenInGame` (`/Game/YohanBlueprints/BP_Checkpoint.Niagara` NextCheckpoint) false false)
  (set `PrimitiveComponent.bGenerateOverlapEvents` true _trigger))

(fn `LapCheck`
  (params (Checkpoint :type Integer))
  (locals (LocalCheckPoint :type Integer))
  (bind _output_get (set `local.LocalCheckPoint` Checkpoint))
  (if (== _output_get (`self.TotalCheckpoints`))
    (bind _isracecomplete (`self.RaceCompleteCheck`))
    (if _isracecomplete
      (`self.ActivateCheckpoint` (`|GetArrayItem` (`self.Checkpoints`)))
      (`/Game/VehicleTemplate/Blueprints/VehiclePlayerController.UpdateLap` (`self.ControllerReference`))
      (set `/Game/VehicleTemplate/Blueprints/VehiclePlayerController.RespawnLocation` (`self.GetTransform` (`|GetArrayItem` (`self.Checkpoints`) (- (`local.LocalCheckPoint`) 1))) (`self.ControllerReference`) :!label _label))
    (else
      (`self.ActivateCheckpoint` (`|GetArrayItem` (`self.Checkpoints`) (`local.LocalCheckPoint`)))
      (goto _label))))

(fn `RaceCompleteCheck`
  (returns (IsRaceComplete :type Boolean))
  (locals (LocalComplete :type Boolean))
  (bind _controllerreference (`self.ControllerReference`))
  (bind _controllerreference_2 (`self.ControllerReference`))
  (if (>= (`/Game/VehicleTemplate/Blueprints/VehiclePlayerController.ActualLap` _controllerreference) (`/Game/VehicleTemplate/Blueprints/VehiclePlayerController.MaxLap` _controllerreference))
    (bind _output_get (set `/Game/VehicleTemplate/Blueprints/VehiclePlayerController.RaceComplete` true _controllerreference_2))
    (set `local.LocalComplete` _output_get)
    (else
      (bind _output_get_2 (set `/Game/VehicleTemplate/Blueprints/VehiclePlayerController.RaceComplete` false _controllerreference_2))
      (set `local.LocalComplete` _output_get_2)))
  (return (`local.LocalComplete`)))

(fn `UpdateTimes`
  (set `/Game/VehicleTemplate/Blueprints/VehiclePlayerController.ActualRaceTime` (`self.ActualRaceTime`) (`self.ControllerReference`)))

(fn `UserConstructionScript`)